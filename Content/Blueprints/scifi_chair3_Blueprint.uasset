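; Sci-fi chair actor that detects the first-person character, with an unfinished E-key interaction.
; Its Trigger component enables input on the chair when the character begins overlap, printing a green debug message, and disables it on end overlap.
; Pressing E hits a FlipFlop with nothing connected to its outputs.
; Teleport and attach-actor nodes are present but unwired, so they never run.
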(event OnComponentEndOverlap(Trigger)
  (params (OverlappedComponent :type Primitive%20Component%20Object%20Reference) (OtherActor :type Actor%20Object%20Reference) (OtherComp :type Primitive%20Component%20Object%20Reference) (OtherBodyIndex :type Integer))
  (Utilities|Casting|CastToFirstPersonCharacter OtherActor)
  (Input|DisableInput (Game|GetPlayerController 0)))

(event OnComponentBeginOverlap(Trigger)
  (params (OverlappedComponent :type Primitive%20Component%20Object%20Reference) (OtherActor :type Actor%20Object%20Reference) (OtherComp :type Primitive%20Component%20Object%20Reference) (OtherBodyIndex :type Integer) (bFromSweep :type Boolean) (SweepResult :type Hit%20Result%20Structure%20%28by%20ref%29))
  (Utilities|Casting|CastToFirstPersonCharacter OtherActor)
  (Input|EnableInput (Game|GetPlayerController 0))
  (Development|PrintString "HELLO AGAIN" true true "(R=0.357114,G=1.000000,B=0.468546,A=1.000000)"))

(event EventBeginPlay)

(event Collision|EventActorBeginOverlap
  (params (OtherActor :type Actor%20Object%20Reference)))

(event EventTick
  (params (DeltaSeconds :type Float%20%28single-precision%29)))

(event Input|KeyboardEvents|E
  (params (Key :type Key%20Structure))
  (:Pressed
    (Utilities|FlowControl|FlipFlop)))

(fn ConstructionScript)